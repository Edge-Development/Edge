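; Inventory component that holds item contents in a fixed number of slots.
; On BeginPlay it resizes the Inventory array to NumberOfSlots.
; AddToInventory passes non-stackable items to CreateStack, which writes them at the index returned by an array Find, apparently searching for an empty slot.
; Stackable items have no handling yet, and the write can grow the array through SizeToFit.
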(event `self.ReceiveBeginPlay`
  (`self.PrepareInventory`))

(fn `Add to Inventory`
  (params (ContentsToAdd :type "/Game/InventorySystem/SlotStructure Structure"))
  (returns (success :type Boolean))
  (if (not (`.Stackable_14_4FB3096F4B0C879498F39790C5A4A96E` (break `/Game/InventorySystem/Item_structure` (break `/Game/InventorySystem/SlotStructure` ContentsToAdd))))
    (`self.CreateStack` self (`local.ContentsToAdd`))
    (return true)))

(fn `CreateStack`
  (params (ContentsToAdd :type "/Game/InventorySystem/SlotStructure Structure"))
  (bind _inventory (`self.Inventory`))
  (`KismetArrayLibrary.Array_Set` _inventory (`KismetArrayLibrary.Array_Find` _inventory) ContentsToAdd true))

(fn `PrepareInventory`
  (`KismetArrayLibrary.Array_Resize` (`self.Inventory`) (`self.Number of slots`)))