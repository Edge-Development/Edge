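; Base item actor that the player can pick up, inspect, drop or throw.
; Interact attaches it to the player's grip point, or starts inspection if an item is already held.
; Inspection moves input to the item and places it before the camera, with toggled mouse or gamepad rotation.
; Throwing applies a physics impulse along control rotation; on impact the item spawns a decal and sound, reports AI noise and destroys itself.
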(event `self.ReceiveHit`
  (params (MyComp :type "PrimitiveComponent Object Reference") (Other :type "Actor Object Reference") (OtherComp :type "PrimitiveComponent Object Reference") (bSelfMoved :type Boolean) (HitLocation :type "Vector Structure") (HitNormal :type "Vector Structure") (NormalImpulse :type "Vector Structure") (Hit :type "HitResult Structure (by ref)"))
  (bind _returnvalue (`KismetMathLibrary.Conv_VectorToRotator` HitNormal))
  ;[0 0.9095 1] Spawning Decal At Impact Loc
  (if (`SceneComponent.IsSimulatingPhysics` (`self.StaticMesh`) "None")
    (if (`self.HasBeenThrown`)
      (`|ExecutionSequence`
        (:`then_0`
          (`GameplayStatics.SpawnDecalAtLocation` "/Game/Images/Materials/Hit.Hit" (200.0 200.0 200.0) HitLocation _returnvalue 0.2)
          (`KismetSystemLibrary.Delay` 0.2))
        (:`then_1`
          (`GameplayStatics.SpawnSoundAtLocation` null HitLocation _returnvalue 0.5 1.0 0.0 null null)
          (`AISense_Hearing.ReportNoiseEvent` HitLocation 1.0 self 0.0 "Noise")))
      (`KismetSystemLibrary.Delay` 0.2)
      (`self.K2_DestroyActor`))))

(event `InputAxisKey|Gamepad_RightY`
  (params (AxisValue :type "Float (single-precision)"))
  ;[0.7344 0 0.02885] Rotation Using Mouse Y-Axis
  (if (`self.IsRotating`)
    (`self.K2_SetActorRotation` (`KismetMathLibrary.ComposeRotators` (`self.K2_GetActorRotation`) (`KismetMathLibrary.MakeRotator` 0.0 (* AxisValue -5.0))))))

(event `InputAxisKey|Gamepad_RightX`
  (params (AxisValue :type "Float (single-precision)"))
  ;[1 0 0.04073] Rotation using Mouse X-axis
  (if (`self.IsRotating`) :!label _label
    (`self.K2_SetActorRotation` (`KismetMathLibrary.ComposeRotators` (`self.K2_GetActorRotation`) (`KismetMathLibrary.MakeRotator` 0.0 0.0 (* AxisValue -5.0))))))

(event `InputAxisKey|MouseX`
  (params (AxisValue :type "Float (single-precision)"))
  ;[1 0 0.04073] Rotation using Mouse X-axis
  (goto _label))

(event `InputAxisKey|MouseY`
  (params (AxisValue :type "Float (single-precision)"))
  ;[0.7344 0 0.02885] Rotation Using Mouse Y-Axis
)

(event `Key|LeftMouseButton`
  (params (Key :type "Key Structure"))
  ;[0.8177 0.004742 0.04377] Setting Rotate Bool
  (:`Pressed`
    (`/Engine/EditorBlueprintResources/StandardMacros.FlipFlop` :!label _label_2
      (:`A`
        (set `self.IsRotating` true))
      (:`B`
        (set `self.IsRotating` false)))))

(event `/Game/Items/Interface/InteractInterface.Interact`
  (params (Player :type "/Game/ThirdPersonBP/Blueprints/ThirdPersonCharacter Object Reference"))
  ;[0.2024 0.3723 1] Enable Interaction
  (bind _output_get (set `self.Player` Player))
  (`/Game/ThirdPersonBP/Blueprints/ThirdPersonCharacter.CurrentHeldItem` _output_get
    (:`then`
      (`self.Start Inspection`))
    (:`else`
      (`self.PickUp`))))

(event `Key|Gamepad_FaceButton_Left`
  (params (Key :type "Key Structure"))
  (:`Pressed`
    (goto _label_2)))

(event `InputAction|Interact`
  (params (Key :type "Key Structure"))
  ;[0.2024 0.3723 1] Enable Interaction
  (:`Pressed`
    (`self.Stop Inspection`)))

(fn `Drop`
  (bind _returnvalue (`GameplayStatics.GetPlayerCameraManager` 0))
  (bind _staticmesh (`self.StaticMesh`))
  (set `self.HasBeenThrown` false)
  (`self.K2_DetachFromActor` "KeepWorld" "KeepWorld" "KeepWorld")
  (`self.K2_SetActorLocation` (+ (`PlayerCameraManager.GetCameraLocation` _returnvalue) (* (`KismetMathLibrary.GetForwardVector` (`PlayerCameraManager.GetCameraRotation` _returnvalue)) 300.0)))
  (`PrimitiveComponent.SetSimulatePhysics` _staticmesh true)
  (`PrimitiveComponent.SetCollisionEnabled` _staticmesh "QueryAndPhysics"))

(fn `PickUp`
  (bind _staticmesh (`self.StaticMesh`))
  (`self.K2_AttachToComponent` (`/Game/ThirdPersonBP/Blueprints/ThirdPersonCharacter.ItemGripPoint` (`self.Player`)) "None" "SnapToTarget" "SnapToTarget" "KeepRelative")
  (`PrimitiveComponent.SetSimulatePhysics` _staticmesh false)
  (`PrimitiveComponent.SetCollisionEnabled` _staticmesh "NoCollision")
  (set `/Game/ThirdPersonBP/Blueprints/ThirdPersonCharacter.CurrentHeldItem` self (`self.Player`)))

(fn `Start Inspection`
  (bind _returnvalue (`GameplayStatics.GetPlayerCameraManager` 0))
  (bind _returnvalue_2 (`GameplayStatics.GetPlayerController` 0))
  (`self.DisableInput` (`self.Player`) _returnvalue_2)
  (`self.EnableInput` _returnvalue_2)
  (`self.K2_SetActorLocation` (+ (`PlayerCameraManager.GetCameraLocation` _returnvalue) (* (`KismetMathLibrary.GetForwardVector` (`PlayerCameraManager.GetCameraRotation` _returnvalue)) 300.0))))

(fn `Stop Inspection`
  (bind _returnvalue (`GameplayStatics.GetPlayerController` 0))
  (`self.DisableInput` _returnvalue)
  (`self.EnableInput` (`self.Player`) _returnvalue)
  (`self.K2_SetActorRelativeLocation` (0.0 0.0 0.0))
  (`self.K2_SetActorRelativeRotation` (struct)))

(fn `Throw`
  (bind _player (`self.Player`))
  (bind _staticmesh (`self.StaticMesh`))
  (set `self.HasBeenThrown` true)
  (`self.K2_DetachFromActor` "KeepWorld" "KeepWorld" "KeepWorld")
  (`self.K2_SetActorLocation` (`SceneComponent.K2_GetComponentLocation` (`/Game/ThirdPersonBP/Blueprints/ThirdPersonCharacter.ItemGripPoint` _player)))
  (`PrimitiveComponent.SetSimulatePhysics` _staticmesh true)
  (`PrimitiveComponent.SetCollisionEnabled` _staticmesh "QueryAndPhysics")
  (`PrimitiveComponent.AddImpulse` (`self.StaticMesh`) (* (`KismetMathLibrary.GetForwardVector` (`Pawn.GetControlRotation` _player)) 20000.0) "None" false))

(fn `UserConstructionScript`)